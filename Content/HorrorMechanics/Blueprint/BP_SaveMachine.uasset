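; BP_SaveMachine is an interactable save machine actor for a horror game that opens a HUD screen with a mouse cursor when used.
; It gets a GUID in the Construction Script and implements checkpoint interface functions that expose that GUID and a freshly created data container.
; Destruction is recorded against the GUID, so loading from a checkpoint destroys the machine again if it was previously destroyed.
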(event EventBeginPlay)

(event Collision|EventActorBeginOverlap
  (params (OtherActor :type Actor%20Object%20Reference)))

(event EventTick
  (params (DeltaSeconds :type Float%20%28single-precision%29)))

(event EventDestroyed
  (CallFunction|SetActorDestroyed (Variables|Actor|GetGUID)))

(event EventLoadfromCheckpoint
  (params (ActorData :type Generic%20Data%20Container%20Struct%20Structure))
  (bind _returnvalue (CallFunction|IsActorDestroyed (Variables|Actor|GetGUID)))
  (if _returnvalue
    (Actor|DestroyActor)))

(event EventInteraction
  (params (PlayerController :type Player%20Controller%20Object%20Reference) (Component :type Actor%20Component%20Object%20Reference))
  (bind _asbp_horror_hud (Utilities|Casting|CastToBP_HorrorHUD (HUD|GetHUD PlayerController)))
  (Default|SetActiveUI _asbp_horror_hud "NewEnumerator7" true))

(fn ConstructionScript
  (CallFunction|SetActorGUID self (Variables|Actor|GetGUID)))

(fn ForceActorGUID
  (params (GUID :type Guid%20Structure))
  (return false))

(fn GetActorGUID
  (return (Variables|Actor|GetGUID)))

(fn GetCheckpointData
  (bind _datacontainer (CallFunction|CreateCheckpointDataContainer))
  (return true (Variables|/Game/HorrorMechanics/Blueprint/SaveSystem/BP_CheckpointDataContainer.BP_CheckpointDataContainer_C|GetDataStruct _datacontainer)))

(fn IsInteractionDisabled
  (params (Component :type Primitive%20Component%20Object%20Reference))
  (return false))
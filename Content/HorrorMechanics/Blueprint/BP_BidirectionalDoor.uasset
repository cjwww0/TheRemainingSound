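; Physics-driven door that swings both ways, extending a parent door class with its own open, close and automatic-close behavior.
; BeginPlay creates a swing-limited hinge constraint; opening enables physics and applies an impulse whose direction depends on the player's side.
; Automatic close disables physics, lerps rotation back via a timeline with a one-shot sound, then resets and locks the door.
; Close acts only without a valid PlayerController, so players cannot close it through that event.
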(event Custom|CloseUsingAnimation
  (bind _closedoor (Variables|Default|GetCloseDoor))
  (bind _defaultdoortransform (Variables|Default|GetDefaultDoorTransform))
  (bind _door (Variables|Default|GetDoor))
  ;[0.2 0.2 0.2 0.2] Close Using Animation
  (if (not (Audio|Components|Audio|IsPlaying _closedoor))
    (Components|Timeline|SetPlayRate _closedoor (Variables|Default|GetCloseSpeed))
    (Physics|SetSimulatePhysics (Variables|Default|GetDoor) false)
    (bind _interpolation (Timeline|CloseDoor PlayFromStart) ; When modifying this curve, make sure it goes from 0.0 to 1.0, both time and value
      (:Update
        (Transformation|SetRelativeRotation _door (Math|Rotator|Lerp(Rotator) (Variables|/Script/Engine.SceneComponent|GetRelativeRotation _door) (.Rotation (Math|Transform|BreakTransform _defaultdoortransform)) _interpolation true) false false)
        (if (Math|Float|NearlyEqual(Float) _interpolation 1.0 0.7)
          (Utilities|FlowControl|DoOnce false :!label _label
            (:Completed
              (Audio|PlaySoundatLocation "/Game/HorrorMechanics/ExampleAssets/Sounds/Doors/SC_DoorClose.SC_DoorClose" (CallFunction|OpenCloseSoundLocation) "0, 0, 0" 0.5 1.0 0.0 "/Game/HorrorMechanics/ExampleAssets/Sounds/SA_Default_01.SA_Default_01" 0 0)))))
      (:Finished
        (Transformation|SetRelativeTransform _door _defaultdoortransform false false)
        (CallFunction|Close 0 false)
        (goto _label Reset)))))

(event EventBeginPlay
  ;[0.2 0.2 0.2 0.2] BeginPlay
  (bind _returnvalue (AddComponent|AddPhysicsConstraintComponent false (Math|Transform|MakeTransform (Math|Vector|MakeVector (.X (Math|Vector|BreakVector (.boxextent (StaticMesh|GetBounds (Variables|/Script/Engine.StaticMeshComponent|GetStaticMesh (Variables|Default|GetDoor)))))) 0.0 0.0) "0,80.000000, 0")))
  (bind _output_get (Variables|Default|SetHinge _returnvalue))
  (Class|PhysicsConstraintComponent|SetAngularSwing1Limit _output_get "ACM_Limited" (Variables|Default|GetSwing1Limit))
  (Variables|Default|SetDefaultDoorTransform (Transformation|GetRelativeTransform (Variables|Default|GetDoor)))
  (|CallParentFunction))

(event EventAutomaticClose
  ;[0.2 0.2 0.2 0.2] Automatic Close
  (CallFunction|CloseUsingAnimation))

(event EventClose
  (params (PlayerController :type Player%20Controller%20Object%20Reference) (PlaySound :type Boolean))
  ;[0.2 0.2 0.2 0.2] Close
  (Utilities|IsValid PlayerController
    (:Is%20Not%20Valid
      (Utilities|FlowControl|Sequence
        (:then_0
          (Transformation|SetRelativeTransform (Variables|Default|GetDoor) (Variables|Default|GetDefaultDoorTransform) false false)
          (Class|PhysicsConstraintComponent|SetAngularSwing1Limit (Variables|Default|GetHinge) "ACM_Locked" 0.0)
          (Physics|SetSimulatePhysics (Variables|Default|GetDoor) false))
        (:then_1
          (|CallParentFunction PlayerController PlaySound))))))

(event EventOpen
  (params (PlayerController :type Player%20Controller%20Object%20Reference) (PlaySound :type Boolean))
  (bind _returnvalue (Pawn|GetControlledPawn PlayerController))
  (bind _returnvalue_2 (Transformation|GetActorLocation))
  (bind _returnvalue_3 (Transformation|GetActorLocation _returnvalue))
  ;[0.2 0.2 0.2 0.2] Open
  (Utilities|FlowControl|Sequence
    (:then_0
      (Physics|SetSimulatePhysics (Variables|Default|GetDoor) true)
      (Class|PhysicsConstraintComponent|SetAngularSwing1Limit (Variables|Default|GetHinge) "ACM_Limited" (Variables|Default|GetSwing1Limit))
      (CallFunction|AddOpenImpulse 1e+04 (< (Math|Vector|DotProduct (Transformation|GetActorRightVector) (Math|Vector|Normalize (- (Math|Vector|MakeVector (.x _returnvalue_2) (.y _returnvalue_2) 0.0) (Math|Vector|MakeVector (.x _returnvalue_3) (.y _returnvalue_3) 0.0)))) 0.0)))
    (:then_1
      (|CallParentFunction PlayerController PlaySound))))

(fn ConstructionScript
  (|CallParentFunction))

(fn AddOpenImpulse
  (params (ImpulseAmount :type Float%20%28single-precision%29) (Forward :type Boolean))
  (bind _door (Variables|Default|GetDoor))
  (Physics|AddImpulseatLocation _door (+ (Transformation|GetActorLocation) (* (Math|Vector|GetRightVector _door) (* ImpulseAmount (select Forward -1.0 1.0)))) (CallFunction|OpenCloseSoundLocation) "None"))
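; Workbench panel puzzle actor for a horror game, where the player places inventory parts until the puzzle completes.
; It delegates item checks, placement and completion to RemainWorkbenchPuzzle, finalizing the puzzle once complete.
; Puzzle mode requests an item choice, or prints a missing-part message when none is usable.
; BeginPlay injects five combined-circle items, and the first-panel-placed event triggers a workshop light fault.
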(event Custom|OnFirstPanelPlaced_Event
  (Utilities|IsValid "/Game/HorrorMechanics/Temporary/BP_WorkshopLightFaultController.BP_WorkshopLightFaultController"
    (:Is%20Valid
      (Class|RemainWorkshopLightFaultController|TriggerFaultState (Variables|Default|GetLightFaultController)))))

(event EventBeginPlay
  (|CallParentFunction)
  (EventDispatchers|AssignOnFirstPanelPlaced (Variables|Default|GetRemainWorkbenchPuzzle) (delegate Custom|OnFirstPanelPlaced_Event))
  (Class|RemainInventoryDebugLibrary|InjectInventoryItems (Utilities|Array|MakeArray "/Game/HorrorMechanics/Database/InventoryItems/BP_CombinedCircle_ItemData.BP_CombinedCircle_ItemData_C" "/Game/HorrorMechanics/Database/InventoryItems/BP_CombinedCircle_ItemData.BP_CombinedCircle_ItemData_C" "/Game/HorrorMechanics/Database/InventoryItems/BP_CombinedCircle_ItemData.BP_CombinedCircle_ItemData_C" "/Game/HorrorMechanics/Database/InventoryItems/BP_CombinedCircle_ItemData.BP_CombinedCircle_ItemData_C" "/Game/HorrorMechanics/Database/InventoryItems/BP_CombinedCircle_ItemData.BP_CombinedCircle_ItemData_C")))

(event Collision|EventActorBeginOverlap
  (params (OtherActor :type Actor%20Object%20Reference)))

(event EventTick
  (params (DeltaSeconds :type Float%20%28single-precision%29))
  (|CallParentFunction DeltaSeconds) ; 此节点被禁用，将不会被调用。\n从引脚连出引线来编译功能。
)

(event EventUseItem
  (params (Item :type Object%20Object%20Reference))
  (bind _returnvalue (Class|RemainWorkbenchPuzzleComponent|PlaceItem (Variables|Default|GetRemainWorkbenchPuzzle) Item (.Inventory (CallFunction|GetInventory))))
  (if _returnvalue
    (if (Class|RemainWorkbenchPuzzleComponent|IsComplete (Variables|Default|GetRemainWorkbenchPuzzle))
      (CallFunction|FinalizePuzzle))))

(event EventPuzzleModeActivated
  (if (Class|RemainPuzzleInventoryLibrary|HasUsableInventoryItemsforPuzzle)
    (CallFunction|RequestChooseItem)
    (else
      (Development|PrintString "缺少当前可放置部件"))))

(fn ConstructionScript
  (|CallParentFunction))

(fn CanUseItem
  (params (PlayerController :type Player%20Controller%20Object%20Reference) (Item :type Object%20Object%20Reference))
  (return (Class|RemainWorkbenchPuzzleComponent|CanUseItem (Variables|Default|GetRemainWorkbenchPuzzle) Item)))
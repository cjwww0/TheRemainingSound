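; BP_Inventory is the player's inventory in the horror game, holding slotted item objects, document objects and virtual keys.
; It adds, swaps, combines (trying both orders) and removes items, opening a replace screen when full, and checks both key types by GUID.
; Wielding waits for the previous actor's unwield event before spawning the next through pawn messages.
; Checkpoint functions save and rebuild everything, muting notifications during loading.
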(event Custom|CharacterUnwield
  ;[0.2 0.2 0.2 0.2] Character: Try to unwield previous item first
  (bind _asbp_horror_game_state (Utilities|Casting|CastToBP_HorrorGameState (Variables|References|GetGameState))
    (:then
      (Utilities|IsValid (Pawn|GetControlledPawn (Default|GetPlayerController _asbp_horror_game_state))
        (:Is%20Valid
          (bind _wieldableactor (Class|BPPlayerCharacterInterface|GetWieldedItem(Message) (Pawn|GetControlledPawn (Default|GetPlayerController _asbp_horror_game_state))))
          (Utilities|IsValid _wieldableactor
            (:Is%20Valid
              (if (== (Utilities|GetClass _wieldableactor) "/Game/HorrorMechanics/Blueprint/Wieldables/BP_PhysicsHandler_WieldableActor.BP_PhysicsHandler_WieldableActor_C")
                (CallFunction|CharacterWield :!label _label)
                (else
                  (Utilities|IsValid _wieldableactor
                    (:Is%20Valid
                      (EventDispatchers|AssignUnwieldedEVD _wieldableactor (delegate Custom|OnPreviousWieldedItemUnwielded))
                      (Default|Unwield _wieldableactor))
                    (:Is%20Not%20Valid
                      (goto _label))))))
            (:Is%20Not%20Valid
              (goto _label))))))
    (:CastFailed
      (goto _label))))

(event Custom|OnPreviousWieldedItemUnwielded
  ;[0.2 0.2 0.2 0.2] Character: Try to unwield previous item first
  (CallFunction|CharacterWield))

(event Custom|WieldItemEv
  (params (Object :type Object%20Object%20Reference))
  ;[0.2 0.2 0.2 0.2] WieldItem
  (Utilities|IsValid Object
    (:Is%20Valid
      (bind _asbp_wieldable_item_data (Utilities|Casting|CastToBP_WieldableItemData Object)
        (:then
          (if (!= Object (Variables|Wielded|GetWieldedItemInstance))
            (Variables|Wielded|SetPreviousWieldedItem (Variables|Wielded|GetWieldedItemInstance))
            (Variables|Wielded|SetWieldedItemInstance Object)
            (Variables|Wielded|SetLastWieldedItemGUID (Variables|/Game/HorrorMechanics/Blueprint/Inventory/BP_InventoryItemAbstractClass.BP_InventoryItemAbstractClass_C|GetGUID _asbp_wieldable_item_data))
            (CallFunction|CharacterUnwield :!label _label)))
        (:CastFailed
          (Variables|Wielded|SetWieldedItemInstance 0 :!label _label_2)
          (goto _label))))
    (:Is%20Not%20Valid
      (goto _label_2))))

(event Custom|CharacterWield
  ;[0.2 0.2 0.2 0.2] Character wield
  (bind _asbp_horror_game_state (Utilities|Casting|CastToBP_HorrorGameState (Variables|References|GetGameState)))
  (Utilities|IsValid (Default|GetPlayerController _asbp_horror_game_state)
    (:Is%20Valid
      (bind _asbp_wieldable_item_data (Utilities|Casting|CastToBP_WieldableItemData (Variables|Wielded|GetWieldedItemInstance))
        (:then
          (bind _childactorref (Class|BPPlayerCharacterInterface|WieldItem(Message) (Pawn|GetControlledPawn (Default|GetPlayerController _asbp_horror_game_state)) (Variables|/Game/HorrorMechanics/Blueprint/Wieldables/BP_WieldableItemData.BP_WieldableItemData_C|GetWieldableActorClass _asbp_wieldable_item_data) (Variables|/Game/HorrorMechanics/Blueprint/Wieldables/BP_WieldableItemData.BP_WieldableItemData_C|GetThirdPersonMesh _asbp_wieldable_item_data)))
          (Variables|/Game/HorrorMechanics/Blueprint/Wieldables/BP_WieldableActor.BP_WieldableActor_C|SetInventoryItemRef _childactorref _asbp_wieldable_item_data)
          (Default|CallItemWieldedEVD _childactorref))
        (:CastFailed
          (Class|BPPlayerCharacterInterface|WieldItem(Message) (Pawn|GetControlledPawn (Default|GetPlayerController _asbp_horror_game_state))) ; Unwield only, as the current item is invalid
        )))))

(fn AddKey
  (params (Name :type String) (KeyGUID :type Guid%20Structure))
  (if (Guid|IsValidGuid KeyGUID)
    (Utilities|Array|Add (Variables|Default|GetVirtualKeys) (Utilities|Struct|MakeVirtualKey_Struct Name KeyGUID))
    (CallFunction|Notify (Utilities|String|Append Name " added to inventory"))))

(fn GetDocument
  (params (Document :type Document%20DT%20Ref%20Struct%20Structure))
  (bind (_rowname _type) (Utilities|Struct|BreakDocumentDT_Ref_Struct Document))
  (switch Utilities|FlowControl|Switch|SwitchonDocumentType_Enum _type
    (:NewEnumerator0
      (bind _returnvalue (Utilities|GetDataTableRow "/Game/HorrorMechanics/Database/Documents/Notes_DataTable.Notes_DataTable" _rowname)
        (:then
          _)))
    (:NewEnumerator1
      (bind _returnvalue_2 (Utilities|GetDataTableRow "/Game/HorrorMechanics/Database/Documents/GenericDocuments_DataTable.GenericDocuments_DataTable" _rowname)
        (:then
          _)))
    (:NewEnumerator2
      (bind _returnvalue_3 (Utilities|GetDataTableRow "/Game/HorrorMechanics/Database/Documents/Books_DataTable.Books_DataTable" _rowname)
        (:then
          _))))
  (return _returnvalue _returnvalue_2 _returnvalue_3 _type))

(fn AddDocumentasDTRef
  (params (DocDT_Ref :type Document%20DT%20Ref%20Struct%20Structure))
  (bind (_rowname _type) (Utilities|Struct|BreakDocumentDT_Ref_Struct DocDT_Ref))
  (bind _returnvalue (Utilities|String|MakeLiteralString " added to documents"))
  (bind _self self)
  (bind _documents (Variables|Default|GetDocuments))
  (switch Utilities|FlowControl|Switch|SwitchonDocumentType_Enum _type
    (:NewEnumerator0
      (bind _returnvalue_2 (Game|ConstructObjectfromClass _self "/Game/HorrorMechanics/Blueprint/Documents/Data/BP_NoteData.BP_NoteData_C" _rowname))
      (bind _returnvalue_3 (Utilities|Array|Add _documents _returnvalue_2))
      (CallFunction|Notify (Utilities|String|Append (Utilities|Struct|BreakNote_Struct (Default|GetStruct _returnvalue_2)) _returnvalue))
      (return _returnvalue_3))
    (:NewEnumerator1
      (bind _returnvalue_4 (Game|ConstructObjectfromClass _self "/Game/HorrorMechanics/Blueprint/Documents/Data/BP_GenericDocumentData.BP_GenericDocumentData_C" _rowname))
      (bind _returnvalue_5 (Utilities|Array|Add _documents _returnvalue_4))
      (CallFunction|Notify (Utilities|String|Append (.Name (Utilities|Struct|BreakGenericDocument_Struct (Default|GetStruct _returnvalue_4))) _returnvalue))
      (return _returnvalue_5))
    (:NewEnumerator2
      (bind _returnvalue_6 (Game|ConstructObjectfromClass _self "/Game/HorrorMechanics/Blueprint/Documents/Data/BP_BookData.BP_BookData_C" _rowname))
      (bind _returnvalue_7 (Utilities|Array|Add _documents _returnvalue_6))
      (CallFunction|Notify (Utilities|String|Append (Utilities|Struct|BreakBook_Struct (Default|GetStruct _returnvalue_6)) _returnvalue))
      (return _returnvalue_7))))

(fn WieldItem
  (params (ItemInstance :type Object%20Object%20Reference))
  (CallFunction|WieldItemEv ItemInstance))

(fn ToggleWieldable
  (Utilities|IsValid (Variables|Wielded|GetWieldedItemInstance)
    (:Is%20Valid
      (Wielded|WieldItem))
    (:Is%20Not%20Valid
      (if (Guid|IsValidGuid (Variables|Wielded|GetLastWieldedItemGUID))
        (bind _array_element (Utilities|Array|ForEachLoopwithBreak (Variables|Items|GetInventoryItems) :!label _label)
          (:LoopBody
            (bind _asbp_wieldable_item_data (Utilities|Casting|CastToBP_WieldableItemData _array_element))
            (if (== (Variables|Wielded|GetLastWieldedItemGUID) (Variables|/Game/HorrorMechanics/Blueprint/Inventory/BP_InventoryItemAbstractClass.BP_InventoryItemAbstractClass_C|GetGUID _array_element))
              (LocalVariables|SetFound _asbp_wieldable_item_data)
              (goto _label Break)))
          (:Completed
            (Utilities|IsValid (LocalVariables|GetFound)
              (:Is%20Valid
                (Wielded|WieldItem (LocalVariables|GetFound))))))))))

(fn CheckforKey
  (params (Key_GUID :type Guid%20Structure) (SetAsUsed :type Boolean))
  (bind _virtualkeys (Variables|Default|GetVirtualKeys))
  (bind _inventoryitems (Variables|Items|GetInventoryItems))
  (if (Guid|IsValidGuid Key_GUID)
    ;[0.2 0.2 0.2 0.2] Check for virtual key
    (bind (_array_element _array_index) (Utilities|Array|ForEachLoopwithBreak _virtualkeys :!label _label)
      (:LoopBody
        (if (== Key_GUID (Utilities|Struct|BreakVirtualKey_Struct _array_element))
          (LocalVariables|SetFoundIndex _array_index)
          (goto _label Break)))
      (:Completed
        (if (== (LocalVariables|GetFoundIndex) -1)
          ;[0.2 0.2 0.2 0.2] Check for examinable key
          (bind (_array_element_2 _array_index_2) (Utilities|Array|ForEachLoopwithBreak _inventoryitems :!label _label_2)
            (:LoopBody
              (bind _asbp_key_item_data (Utilities|Casting|CastToBP_Key_ItemData _array_element_2))
              (if (== Key_GUID (Variables|/Game/HorrorMechanics/Blueprint/Keys/BP_Key_ItemData.BP_Key_ItemData_C|GetKeyGUID _asbp_key_item_data))
                (LocalVariables|SetFoundIndex _array_index_2)
                (goto _label_2 Break)))
            (:Completed
              (if (== (LocalVariables|GetFoundIndex) -1)
                (return false false "" "NewEnumerator0" -1)
                (else
                  (bind _asbp_key_item_data_2 (Utilities|Casting|CastToBP_Key_ItemData (Utilities|Array|Get(acopy) _inventoryitems (LocalVariables|GetFoundIndex))))
                  (LocalVariables|SetPreviouslyUsed (Variables|/Game/HorrorMechanics/Blueprint/Keys/BP_Key_ItemData.BP_Key_ItemData_C|GetHasBeenUsed _asbp_key_item_data_2))
                  (if SetAsUsed
                    (Default|UseKey _asbp_key_item_data_2))
                  (return true (LocalVariables|GetPreviouslyUsed) (Variables|/Game/HorrorMechanics/Blueprint/Inventory/BP_InventoryItemAbstractClass.BP_InventoryItemAbstractClass_C|GetName _asbp_key_item_data_2) "NewEnumerator2" (LocalVariables|GetFoundIndex))))))
          (else
            (LocalVariables|SetPreviouslyUsed (.HasBeenUsed (Utilities|Struct|BreakVirtualKey_Struct (Utilities|Array|Get(acopy) _virtualkeys (LocalVariables|GetFoundIndex)))))
            (if SetAsUsed
              (Utilities|Struct|SetmembersinVirtualKey_Struct (Utilities|Array|Get(acopy) _virtualkeys (LocalVariables|GetFoundIndex)) true))
            (return true (LocalVariables|GetPreviouslyUsed) (.Name (Utilities|Struct|BreakVirtualKey_Struct (Utilities|Array|Get(acopy) _virtualkeys (LocalVariables|GetFoundIndex)))) "NewEnumerator1" (LocalVariables|GetFoundIndex))))))
    (else
      (return false false "" "NewEnumerator1" -1))))

(fn GetInventoryItembyIndex
  (params (Index :type Integer))
  (bind _inventoryitems (Variables|Items|GetInventoryItems))
  (bind _output (Utilities|Array|Get(acopy) _inventoryitems Index))
  (if (Utilities|Array|IsValidIndex _inventoryitems Index)
    (Utilities|IsValid _output
      (:Is%20Valid
        (return _output (Utilities|IsValid _output)))
      (:Is%20Not%20Valid
        _)))
  (return 0 false))

(fn CombineItems
  (params (A :type BP%20Inventory%20Item%20Abstract%20Class%20Object%20Reference) (B :type BP%20Inventory%20Item%20Abstract%20Class%20Object%20Reference))
  (LocalVariables|SetA_Item A)
  (LocalVariables|SetB_Item B)
  (Utilities|IsValid (LocalVariables|GetA_Item) :!label _label
    (:Is%20Valid
      (Utilities|IsValid (LocalVariables|GetB_Item)
        (:Is%20Valid
          (bind (_combinedintonewitemclass _combinedsuccessfully _discard) (Default|Combine (LocalVariables|GetA_Item) (LocalVariables|GetB_Item)))
          (if _combinedsuccessfully
            (if (Utilities|IsValidClass _combinedintonewitemclass)
              ;[0.2 0.2 0.2 0.2] New item was created, find best slot
              (LocalVariables|SetNSlot (Utilities|Select :Index _discard :NewEnumerator0 -1 :NewEnumerator1 (Variables|/Game/HorrorMechanics/Blueprint/Inventory/BP_InventoryItemAbstractClass.BP_InventoryItemAbstractClass_C|GetSlot (LocalVariables|GetA_Item)) :NewEnumerator2 (Variables|/Game/HorrorMechanics/Blueprint/Inventory/BP_InventoryItemAbstractClass.BP_InventoryItemAbstractClass_C|GetSlot (LocalVariables|GetB_Item)) :NewEnumerator3 (select (LocalVariables|GetB_to_A) (Variables|/Game/HorrorMechanics/Blueprint/Inventory/BP_InventoryItemAbstractClass.BP_InventoryItemAbstractClass_C|GetSlot (LocalVariables|GetA_Item)) (Variables|/Game/HorrorMechanics/Blueprint/Inventory/BP_InventoryItemAbstractClass.BP_InventoryItemAbstractClass_C|GetSlot (LocalVariables|GetB_Item)))))
              (switch Utilities|FlowControl|Switch|SwitchonABOptions_Enum _discard
                (:NewEnumerator0
                  _)
                (:NewEnumerator1
                  (Items|RemoveInventoryItem (LocalVariables|GetA_Item)))
                (:NewEnumerator2
                  (Items|RemoveInventoryItem (LocalVariables|GetB_Item)))
                (:NewEnumerator3
                  (Items|RemoveInventoryItem (LocalVariables|GetA_Item))
                  (Items|RemoveInventoryItem (LocalVariables|GetB_Item))))
              (bind _inventoryitem (Items|AddItem :ItemClass _combinedintonewitemclass :OptionalSlotIndex (LocalVariables|GetNSlot)))
              (Default|CallNewCombinedItemEVD _inventoryitem)
              (return true _discard)
              (else
                ;[0.2 0.2 0.2 0.2] No new item is created
                (switch Utilities|FlowControl|Switch|SwitchonABOptions_Enum _discard
                  (:NewEnumerator0
                    (return true "NewEnumerator0"))
                  (:NewEnumerator1
                    (Items|RemoveInventoryItem (LocalVariables|GetA_Item)))
                  (:NewEnumerator2
                    (Items|RemoveInventoryItem (LocalVariables|GetB_Item)))
                  (:NewEnumerator3
                    (Items|RemoveInventoryItem (LocalVariables|GetA_Item))
                    (Items|RemoveInventoryItem (LocalVariables|GetB_Item))))
                (return true _discard)))
            (else
              ;[0.2 0.2 0.2 0.2] Try to combine B to A as well, so we don't need to implement it twice in both blueprints
              (if (not (LocalVariables|GetB_to_A))
                (LocalVariables|SetA_Item B)
                (LocalVariables|SetB_Item A)
                (LocalVariables|SetB_to_A true)
                (goto _label)))))
        (:Is%20Not%20Valid
          (return false "NewEnumerator0"))))
    (:Is%20Not%20Valid
      (return false "NewEnumerator0"))))

(fn CombineItemsbyIndex
  (params (A :type Integer) (B :type Integer))
  (bind _inventoryitems (Variables|Items|GetInventoryItems))
  (if (and (Utilities|Array|IsValidIndex _inventoryitems B) (Utilities|Array|IsValidIndex _inventoryitems A))
    (bind _success (Items|CombineItems (Utilities|Array|Get(acopy) _inventoryitems A) (Utilities|Array|Get(acopy) _inventoryitems B)))
    (return _success)
    (else
      (return false))))

(fn SwapItemsbySlot
  (params (A :type Integer) (B :type Integer))
  (Utilities|FlowControl|Sequence
    (:then_0
      (bind _inventoryitem (Items|GetItematSlot A))
      (LocalVariables|SetItemA _inventoryitem))
    (:then_1
      (bind _inventoryitem_2 (Items|GetItematSlot B))
      (LocalVariables|SetItemB _inventoryitem_2))
    (:then_2
      (Utilities|IsValid (LocalVariables|GetItemA)
        (:Is%20Valid
          (Default|SetSlotIndex (LocalVariables|GetItemA) B))))
    (:then_3
      (Utilities|IsValid (LocalVariables|GetItemB)
        (:Is%20Valid
          (Default|SetSlotIndex (LocalVariables|GetItemB) A))))
    (:then_4
      (return true))))

(fn FindFreeSlot
  (bind _index (Items|GetHighestSlotinUse))
  (if (!= _index -1)
    (bind _index_2 (Utilities|FlowControl|ForLoopwithBreak 0 _index :!label _label)
      (:LoopBody
        (bind _valid (Items|GetItematSlot _index_2)) ; if there's a slot not being used
        (if (not _valid)
          (LocalVariables|Set_Index _index_2)
          (goto _label Break)))
      (:Completed
        (if (== (LocalVariables|Get_Index) -1) :!label _label_2
          (LocalVariables|Set_Index (+ _index 1)))
        (return (LocalVariables|Get_Index) (!= (LocalVariables|Get_Index) -1))))
    (else
      (goto _label_2))))

(fn GetItematSlot
  (params (SlotIndex :type Integer))
  (if (!= SlotIndex -1)
    (bind _array_element (Utilities|Array|ForEachLoopwithBreak (Variables|Items|GetInventoryItems) :!label _label)
      (:LoopBody
        (if (== SlotIndex (Variables|/Game/HorrorMechanics/Blueprint/Inventory/BP_InventoryItemAbstractClass.BP_InventoryItemAbstractClass_C|GetSlot _array_element))
          (LocalVariables|SetFound _array_element)
          (goto _label Break)))
      (:Completed
        (return (LocalVariables|GetFound) (Utilities|IsValid (LocalVariables|GetFound)))))
    (else
      (return 0 false))))

(fn SwapItemsbySlotasRef
  (params (A :type BP%20Inventory%20Item%20Abstract%20Class%20Object%20Reference) (B :type BP%20Inventory%20Item%20Abstract%20Class%20Object%20Reference))
  (bind _inventoryitems (Variables|Items|GetInventoryItems))
  (bind _success (Items|SwapItemsbySlot (Utilities|Array|FindItem _inventoryitems A) (Utilities|Array|FindItem _inventoryitems B)))
  (return _success))

(fn RemoveInventoryItem
  (params (InventoryItem :type BP%20Inventory%20Item%20Abstract%20Class%20Object%20Reference))
  (Default|CallItemRemovedEVD InventoryItem)
  (bind _returnvalue (Utilities|Array|RemoveItem (Variables|Items|GetInventoryItems) InventoryItem))
  (Default|CallItemsChangedEVD)
  (return _returnvalue))

(fn GetAllItemsOfClass
  (params (Class :type Object%20Class%20Reference))
  (for _array_element (Variables|Items|GetInventoryItems)
    (if (== Class (Utilities|GetClass _array_element))
      (Utilities|Array|AddUnique (LocalVariables|GetItemsFound) _array_element)))
  (return (LocalVariables|GetItemsFound)))

(fn NewInventoryItemGUID
  (LocalVariables|SetNewGUID (Guid|NewGuid))
  (bind _array_element (Utilities|Array|ForEachLoopwithBreak (Variables|Items|GetInventoryItems) :!label _label)
    (:LoopBody
      (if (== (Variables|/Game/HorrorMechanics/Blueprint/Inventory/BP_InventoryItemAbstractClass.BP_InventoryItemAbstractClass_C|GetGUID _array_element) (LocalVariables|GetNewGUID))
        (LocalVariables|SetFound true)
        (goto _label Break)))
    (:Completed
      (if (LocalVariables|GetFound)
        (return (Guid|NewGuid))
        (else
          (return (LocalVariables|GetNewGUID)))))))

(fn GetCheckpointData
  (bind _documentlist (LocalVariables|GetDocumentList))
  (Utilities|FlowControl|Sequence
    (:then_0
      ;[0.2 0.2 0.2 0.2] Wielded item
      (bind _asbp_wieldable_item_data (Utilities|Casting|CastToBP_WieldableItemData (Variables|Wielded|GetWieldedItemInstance)))
      (LocalVariables|SetWieldedItemGUID (Variables|/Game/HorrorMechanics/Blueprint/Inventory/BP_InventoryItemAbstractClass.BP_InventoryItemAbstractClass_C|GetGUID _asbp_wieldable_item_data))
      (LocalVariables|SetIsWieldingEquipedItem (Variables|/Game/HorrorMechanics/Blueprint/Wieldables/BP_WieldableItemData.BP_WieldableItemData_C|GetIsWielded _asbp_wieldable_item_data)))
    (:then_1
      ;[0.2 0.2 0.2 0.2] Inventory list
      (for _array_element (Variables|Items|GetInventoryItems)
        (bind _savestruct (Default|GetCheckpointData _array_element))
        (Utilities|Array|Add (LocalVariables|GetInventoryListData) (Utilities|Struct|MakeInventoryItemCheckpointData_Struct (Utilities|GetClass _array_element) (select (Guid|IsValidGuid (Variables|/Game/HorrorMechanics/Blueprint/Inventory/BP_InventoryItemAbstractClass.BP_InventoryItemAbstractClass_C|GetGUID _array_element)) (Variables|/Game/HorrorMechanics/Blueprint/Inventory/BP_InventoryItemAbstractClass.BP_InventoryItemAbstractClass_C|GetGUID _array_element) (Guid|NewGuid)) (Variables|/Game/HorrorMechanics/Blueprint/Inventory/BP_InventoryItemAbstractClass.BP_InventoryItemAbstractClass_C|GetSlot _array_element) (Variables|/Game/HorrorMechanics/Blueprint/Inventory/BP_InventoryItemAbstractClass.BP_InventoryItemAbstractClass_C|GetQuantity _array_element) _savestruct))))
    (:then_2
      ;[0.2 0.2 0.2 0.2] Documents
      (for _array_element_2 (Variables|Default|GetDocuments)
        (bind _asbp_note_data (Utilities|Casting|CastToBP_NoteData _array_element_2)
          (:then
            (Utilities|Array|Add _documentlist (Utilities|Struct|MakeDocumentDT_Ref_Struct (Variables|/Game/HorrorMechanics/Blueprint/Documents/Data/BP_NoteData.BP_NoteData_C|GetDataTableRowName _asbp_note_data) "NewEnumerator0")))
          (:CastFailed
            (bind _asbp_generic_document_data (Utilities|Casting|CastToBP_GenericDocumentData _array_element_2)
              (:then
                (Utilities|Array|Add _documentlist (Utilities|Struct|MakeDocumentDT_Ref_Struct (Variables|/Game/HorrorMechanics/Blueprint/Documents/Data/BP_GenericDocumentData.BP_GenericDocumentData_C|GetDataTableRowName _asbp_generic_document_data) "NewEnumerator1")))
              (:CastFailed
                (bind _asbp_book_data (Utilities|Casting|CastToBP_BookData _array_element_2))
                (Utilities|Array|Add _documentlist (Utilities|Struct|MakeDocumentDT_Ref_Struct (Variables|/Game/HorrorMechanics/Blueprint/Documents/Data/BP_BookData.BP_BookData_C|GetDataTableRowName _asbp_book_data) "NewEnumerator2"))))))))
    (:then_3
      (return (Utilities|Struct|MakeInventoryCheckpointData_Struct (LocalVariables|GetInventoryListData) (LocalVariables|GetWieldedItemGUID) (LocalVariables|GetIsWieldingEquipedItem) (LocalVariables|GetDocumentList) (Variables|Default|GetVirtualKeys) (Variables|Items|GetMaxInventoryItems))))))

(fn LoadfromCheckpoint
  (params (InventoryCheckpointData :type Inventory%20Checkpoint%20Data%20Struct%20Structure))
  (bind (_inventoryitems _equipeditemguid _isequipeditemwielded _documents _virtualkeys _maxinventoryitems) (Utilities|Struct|BreakInventoryCheckpointData_Struct InventoryCheckpointData))
  (Utilities|FlowControl|Sequence
    (:then_0
      (Variables|Default|SetIsLoading true))
    (:then_1
      (Utilities|FlowControl|Sequence
        (:then_0
          (Variables|Items|SetMaxInventoryItems _maxinventoryitems))
        (:then_1
          (Variables|Default|SetVirtualKeys _virtualkeys)
          (LocalVariables|SetWielded _isequipeditemwielded)
          (Variables|Wielded|SetLastWieldedItemGUID _equipeditemguid))
        (:then_2
          (for _array_element _inventoryitems
            (bind _asbp_inventory_item_abstract_class (Utilities|Casting|CastToBP_InventoryItemAbstractClassClass (.Class (Utilities|Struct|BreakInventoryItemCheckpointData_Struct _array_element))))
            (Utilities|FlowControl|Sequence
              (:then_0
                (bind _inventoryitem (Items|AddItem _asbp_inventory_item_abstract_class (.GUID (Utilities|Struct|BreakInventoryItemCheckpointData_Struct _array_element)) (.SlotIndex (Utilities|Struct|BreakInventoryItemCheckpointData_Struct _array_element))))
                (Variables|/Game/HorrorMechanics/Blueprint/Inventory/BP_InventoryItemAbstractClass.BP_InventoryItemAbstractClass_C|SetQuantity _inventoryitem (.Quantity (Utilities|Struct|BreakInventoryItemCheckpointData_Struct _array_element))))
              (:then_1
                (Default|LoadfromCheckpoint _inventoryitem (.Data (Utilities|Struct|BreakInventoryItemCheckpointData_Struct _array_element))))
              (:then_2
                (if (== _equipeditemguid (.GUID (Utilities|Struct|BreakInventoryItemCheckpointData_Struct _array_element)))
                  (if (LocalVariables|GetWielded)
                    (bind _asbp_item_data (Utilities|Casting|CastToBP_ItemData _inventoryitem))
                    (Wielded|WieldItem _asbp_item_data)))))))
        (:then_3
          (for _array_element_2 _documents
            (Documents|AddDocumentasDTRef _array_element_2)))))
    (:then_2
      (Variables|Default|SetIsLoading false))))

(fn UseItematSlot
  (params (Slot :type Integer))
  (bind (_inventoryitem _valid) (Items|GetItematSlot Slot))
  (if _valid
    (Default|Use _inventoryitem)))

(fn Notify
  (params (String :type String))
  (if (not (Variables|Default|GetIsLoading))
    (bind _asbp_horror_game_state (Utilities|Casting|CastToBP_HorrorGameState (Variables|References|GetGameState)))
    (Default|Notify _asbp_horror_game_state String)))

(fn AddItem
  (params (ItemClass :type BP%20Inventory%20Item%20Abstract%20Class%20Class%20Reference) (Optional_GUID :type Guid%20Structure) (OptionalSlotIndex :type Integer))
  (bind _maxinventoryitems (Variables|Items|GetMaxInventoryItems))
  (if (Items|IsFull)
    (if (Variables|Default|GetIsLoading) :!label _label
      (Development|PrintString 0 "Error: Inventory is full (MaxInventoryItems)" false true "(R=1.000000,G=0.200000,B=0.000000,A=1.000000)" 0.0)
      (else
        (if (!= (Variables|Items|GetMaxInventoryItems) 0)
          (Items|RequestItemReplace ItemClass Optional_GUID OptionalSlotIndex) ; Inventory is full, show the UI so the user can replace some other item by this new one
        )
        (return 0 false true)))
    (elif (Utilities|IsValidClass ItemClass)
      (Utilities|FlowControl|Sequence
        (:then_0
          (bind (_index _valid) (Items|FindFreeSlot))
          (if _valid
            (LocalVariables|SetFreeSlot _index)))
        (:then_1
          (if (!= (LocalVariables|GetFreeSlot) -1)
            (bind _returnvalue (Game|ConstructObjectfromClass self ItemClass (Variables|References|GetGameState) "NewEnumerator1" (select (Guid|IsValidGuid Optional_GUID) Optional_GUID (Items|NewInventoryItemGUID))))
            (Utilities|Array|AddUnique (Variables|Items|GetInventoryItems) _returnvalue)
            ;[0.2 0.2 0.2 0.2] Set Slot
            (if (or (== OptionalSlotIndex -1) (and (!= _maxinventoryitems -1) (> OptionalSlotIndex _maxinventoryitems))) ; No provided index or beyond MaxInventoryItems
              ;;[0.2 0.2 0.2 0.2] Use a free slot
              (Default|SetSlotIndex _returnvalue (LocalVariables|GetFreeSlot) :!label _label_2)
              (else
                (bind _valid_2 (Items|GetItematSlot OptionalSlotIndex))
                (if _valid_2
                  (goto _label_2)
                  (else
                    (Default|SetSlotIndex _returnvalue OptionalSlotIndex) ; Use provided index
                  ))))
            (Default|CallItemAddedEVD _returnvalue)
            (Default|CallItemsChangedEVD)
            (CallFunction|Notify (Utilities|String|Append (Variables|/Game/HorrorMechanics/Blueprint/Inventory/BP_InventoryItemAbstractClass.BP_InventoryItemAbstractClass_C|GetName _returnvalue) " added to inventory"))
            (return _returnvalue true false)
            (else
              (goto _label)))))
      (else
        (return 0 false false)))))

(fn IsFull
  (bind _maxinventoryitems (Variables|Items|GetMaxInventoryItems))
  (return (and (not (< _maxinventoryitems 0)) (>= (Utilities|Array|Length (Variables|Items|GetInventoryItems)) _maxinventoryitems))))

(fn RequestItemReplace
  (params (ItemClass :type BP%20Inventory%20Item%20Abstract%20Class%20Class%20Reference) (OptionalGUID :type Guid%20Structure) (OptionalSlotIndex :type Integer))
  (bind _asbp_horror_game_state (Utilities|Casting|CastToBP_HorrorGameState (Variables|References|GetGameState)))
  (bind _asbp_horror_hud (Utilities|Casting|CastToBP_HorrorHUD (HUD|GetHUD (Default|GetPlayerController _asbp_horror_game_state))))
  (Default|SetActiveUI _asbp_horror_hud "NewEnumerator6" true)
  (bind _asui_replace_item_screen (Utilities|Casting|CastToUI_ReplaceItemScreen (Variables|/Game/HorrorMechanics/Blueprint/UI/BP_HorrorHUD.BP_HorrorHUD_C|GetReplaceItemScreen _asbp_horror_hud)))
  (Variables|/Game/HorrorMechanics/Blueprint/Inventory/UI/UI_ReplaceItemScreen.UI_ReplaceItemScreen_C|SetItemClass _asui_replace_item_screen ItemClass)
  (Variables|/Game/HorrorMechanics/Blueprint/Inventory/UI/UI_ReplaceItemScreen.UI_ReplaceItemScreen_C|SetOptionalItemGUID _asui_replace_item_screen OptionalGUID)
  (Default|SelectSlot _asui_replace_item_screen OptionalSlotIndex))

(fn GetHighestSlotinUse
  (for _array_element (Variables|Items|GetInventoryItems)
    (if (> (Variables|/Game/HorrorMechanics/Blueprint/Inventory/BP_InventoryItemAbstractClass.BP_InventoryItemAbstractClass_C|GetSlot _array_element) (LocalVariables|GetHighest))
      (LocalVariables|SetHighest (Variables|/Game/HorrorMechanics/Blueprint/Inventory/BP_InventoryItemAbstractClass.BP_InventoryItemAbstractClass_C|GetSlot _array_element))))
  (return (LocalVariables|GetHighest)))
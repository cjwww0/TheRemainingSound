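; Inventory item data Blueprint for the horror game, with empty hooks for construction, examine, collection and reset, and a fixed interact action.
; Its Discard override runs the parent logic and, on success with DropTheItemOnDiscard set, has BP_HorrorGameState spawn a dropped item at the player character's feet.
; The spawn passes the item's class, quantity, checkpoint data and GUID, so the dropped item carries over its identity and state.
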(event Custom|OnConstruct)

(event Custom|OnExamine)

(event Custom|OnCollected
  (params (PlayerController :type Player%20Controller%20Object%20Reference) (ExaminableObjectRef :type Object%20Object%20Reference)))

(event Custom|OnReset)

(fn OnInteractAction
  (return "NewEnumerator0"))

(fn Discard
  (bind _droptheitemondiscard (Variables|Default|GetDropTheItemOnDiscard))
  (bind _success (|CallParentFunction))
  (if _success
    (Utilities|FlowControl|Sequence
      (:then_0
        (if _droptheitemondiscard
          ;[0.2 0.2 0.2 0.2] Spawn Dropped Item
          (bind _asbp_horror_game_state (Utilities|Casting|CastToBP_HorrorGameState (Variables|Default|GetGameState)))
          (bind _ascharacter (Utilities|Casting|CastToCharacter (Pawn|GetControlledPawn (Default|GetPlayerController _asbp_horror_game_state))))
          (bind _savestruct (CallFunction|GetCheckpointData))
          (Default|SpawnDroppedItem _asbp_horror_game_state (Math|Transform|MakeTransform (- (Transformation|GetActorLocation _ascharacter) (Math|Vector|MakeVector 0.0 0.0 (Variables|/Script/Engine.CapsuleComponent|GetCapsuleHalfHeight (Variables|/Script/Engine.Character|GetCapsuleComponent _ascharacter))))) (Utilities|GetClass self) (Variables|Default|GetQuantity) _savestruct (Variables|Default|GetGUID))))
      (:then_1
        (return _success _droptheitemondiscard)))))